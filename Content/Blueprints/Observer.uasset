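; Observer camera pawn for viewing a solar system, with free WASD movement and mouse-wheel zoom.
; Tick applies movement relative to the camera arm and glides the pawn toward ActorSelected, which any movement key clears.
; Wheel input and per-body events for the Sun and planets set TargetArmLength, which Tick interpolates and clamps onto the arm.
; SpaceBar only sets a flag, as the camera transition code is unconnected.
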(event OnComponentBeginOverlap(Sphere1)
  (params (OtherActor :type Actor%20Object%20Reference) (OtherComp :type Primitive%20Component%20Object%20Reference) (OtherBodyIndex :type Integer) (bFromSweep :type Boolean) (SweepResult :type Hit%20Result%20Structure%20%28by%20ref%29))
  ;[1 1 1] CameraZoom
  (Variables|Default|SetZoomEnable false))

(event OnComponentEndOverlap(Sphere1)
  (params (OtherActor :type Actor%20Object%20Reference) (OtherComp :type Primitive%20Component%20Object%20Reference) (OtherBodyIndex :type Integer))
  ;[1 1 1] CameraZoom
  (Variables|Default|SetZoomEnable true))

(event Custom|Earth%20Target%20Lenght
  (Variables|Default|SetTargetArmLength 1.5e+03))

(event Custom|Venus%20Target%20Lengh
  (Variables|Default|SetTargetArmLength 1.45e+03))

(event Custom|Mars%20Target%20Lenght
  (Variables|Default|SetTargetArmLength 1e+03))

(event Custom|Jupiter%20Target%20Lenght
  (Variables|Default|SetTargetArmLength 1.85e+03))

(event Custom|Saturn%20Target%20Lenght
  (Variables|Default|SetTargetArmLength 1.6e+03))

(event Custom|Uranus%20Target%20Lenght
  (Variables|Default|SetTargetArmLength 1.2e+03))

(event Custom|Nepturn%20TARGET%20Lenght
  (Variables|Default|SetTargetArmLength 1.2e+03))

(event Custom|Sun%20Target%20Lenght
  (Variables|Default|SetTargetArmLength 5e+03))

(event Custom|Pluto%20Target%20Lenght
  (Variables|Default|SetTargetArmLength 3e+02))

(event Custom|Mercury%20Target%20Lengh
  (Variables|Default|SetTargetArmLength 9e+02))

(event EventTick
  (params (DeltaSeconds :type Float%20%28single-precision%29))
  (bind _cameraarm (Variables|Default|Getcameraarm))
  (bind _cameraarm_2 (Variables|Default|Getcameraarm))
  (bind _cameraarm_3 (Variables|Default|Getcameraarm))
  (bind _returnvalue (Transformation|GetWorldTransform _cameraarm_2))
  (bind _returnvalue_2 (Transformation|GetWorldTransform _cameraarm_3))
  (bind _rotation (Math|Transform|BreakTransform _returnvalue))
  (bind _rotation_2 (Math|Transform|BreakTransform _returnvalue_2))
  (bind _returnvalue_3 (Math|Vector|GetForwardVector _rotation))
  (bind _returnvalue_4 (Math|Vector|GetForwardVector _rotation_2))
  (bind (_x _y) (Math|Vector|BreakVector _returnvalue_4))
  (bind _returnvalue_5 (* _returnvalue_3 -1e+01))
  (bind (_x_2 _y_2) (Math|Vector|BreakVector _returnvalue_5))
  (Utilities|FlowControl|Sequence
    (:then_0
      (if true
        ;[1 1 1] Camera Movement
        ;;[1 1 1] Move Left
        (Utilities|FlowControl|Sequence
          (:then_0
            (if (Variables|Default|GetMoveLeft)
              (Pawn|Input|AddMovementInput (* (Math|Vector|GetRightVector (.Rotation (Math|Transform|BreakTransform (Transformation|GetWorldTransform (Variables|Default|Getcameraarm))))) -1.0) 1.0 false))
            ;;[1 1 1] Move Right
            (if (Variables|Default|GetMoveRight)
              (Pawn|Input|AddMovementInput (Math|Vector|GetRightVector (.Rotation (Math|Transform|BreakTransform (Transformation|GetWorldTransform (Variables|Default|Getcameraarm))))) 1.0 false))
            ;;[1 1 1] Move Forward
            (if (Variables|Default|GetForward)
              (Pawn|Input|AddMovementInput (Math|Vector|Normalize (Math|Vector|MakeVector _x _y 0.0)) 1.0 false))
            ;;[1 1 1] Move Back
            (if (Variables|Default|GetBack)
              (Pawn|Input|AddMovementInput (Math|Vector|Normalize (Math|Vector|MakeVector _x_2 _y_2 0.0)) 1.0 false))))))
    (:then_1
      (Utilities|IsValid (Variables|Default|GetActorSelected)
        (:Is%20Valid
          (Transformation|SetActorLocation (Math|Interpolation|VInterpTo (Transformation|GetActorLocation) (Transformation|GetActorLocation (Variables|Default|GetActorSelected)) DeltaSeconds 4.0) false false))))
    (:then_2
      ;[1 1 1] Updating Arm Lengh Target
      (if true
        (Variables|/Script/Engine.SpringArmComponent|SetTargetArmLength _cameraarm (Math|Float|Clamp(Float) (Math|Interpolation|FInterpTo (Variables|/Script/Engine.SpringArmComponent|GetTargetArmLength _cameraarm) (Variables|Default|GetTargetArmLength) (Utilities|Time|GetWorldDeltaSeconds) 4.0) 9e+02 5.5e+03))))))

(event Input|KeyboardEvents|SpaceBar
  (params (Key :type Key%20Structure :default "AnyKey"))
  (:Pressed
    (Variables|Default|SetPressSpace true)))

(event Input|MouseEvents|MouseWheelDown
  (params (Key :type Key%20Structure :default "AnyKey"))
  ;[1 1 1] CameraZoom
  (:Pressed
    (if (Variables|Default|GetZoomEnable)
      _
      (else
        (Variables|Default|SetTargetArmLength (Variables|/Script/Engine.SpringArmComponent|GetTargetArmLength (Variables|Default|Getcameraarm)))
        (Variables|Default|SetZoomEnable false)))
    (Variables|Default|SetZoomEnable true)
    (Variables|Default|SetTargetArmLength (- (Variables|Default|GetTargetArmLength) -2.5e+02))))

(event Input|MouseEvents|MouseWheelUp
  (params (Key :type Key%20Structure :default "AnyKey"))
  ;[1 1 1] CameraZoom
  (:Pressed
    (Variables|Default|SetTargetArmLength (- (Variables|Default|GetTargetArmLength) 2.5e+02))))

(event Input|KeyboardEvents|A
  (params (Key :type Key%20Structure :default "AnyKey"))
  (bind _cameraarm (Variables|Default|Getcameraarm))
  (bind _cameraarm_2 (Variables|Default|Getcameraarm))
  (bind _returnvalue (Transformation|GetWorldTransform _cameraarm))
  (bind _returnvalue_2 (Transformation|GetWorldTransform _cameraarm_2))
  (bind _rotation (Math|Transform|BreakTransform _returnvalue))
  (bind _rotation_2 (Math|Transform|BreakTransform _returnvalue_2))
  (bind _returnvalue_3 (Math|Vector|GetForwardVector _rotation))
  (bind _returnvalue_4 (Math|Vector|GetForwardVector _rotation_2))
  (bind (_x _y) (Math|Vector|BreakVector _returnvalue_4))
  (bind _returnvalue_5 (* _returnvalue_3 -1e+01))
  (bind (_x_2 _y_2) (Math|Vector|BreakVector _returnvalue_5))
  ;[1 1 1] Camera Movement
  ;;[1 1 1] Move Left
  (:Pressed
    (Variables|Default|SetMoveLeft true)
    (Variables|Default|SetActorSelected 0)
    (Pawn|Input|AddMovementInput (* (Math|Vector|GetRightVector (.Rotation (Math|Transform|BreakTransform (Transformation|GetWorldTransform (Variables|Default|Getcameraarm))))) -1.0) 1.0 false)
    ;;[1 1 1] Move Right
    (if (Variables|Default|GetMoveRight)
      (Pawn|Input|AddMovementInput (Math|Vector|GetRightVector (.Rotation (Math|Transform|BreakTransform (Transformation|GetWorldTransform (Variables|Default|Getcameraarm))))) 1.0 false))
    ;;[1 1 1] Move Forward
    (if (Variables|Default|GetForward)
      (Pawn|Input|AddMovementInput (Math|Vector|Normalize (Math|Vector|MakeVector _x _y 0.0)) 1.0 false))
    ;;[1 1 1] Move Back
    (if (Variables|Default|GetBack)
      (Pawn|Input|AddMovementInput (Math|Vector|Normalize (Math|Vector|MakeVector _x_2 _y_2 0.0)) 1.0 false)))
  (:Released
    (Variables|Default|SetMoveLeft false)))

(event Input|KeyboardEvents|D
  (params (Key :type Key%20Structure :default "AnyKey"))
  (bind _cameraarm (Variables|Default|Getcameraarm))
  (bind _cameraarm_2 (Variables|Default|Getcameraarm))
  (bind _returnvalue (Transformation|GetWorldTransform _cameraarm))
  (bind _returnvalue_2 (Transformation|GetWorldTransform _cameraarm_2))
  (bind _rotation (Math|Transform|BreakTransform _returnvalue))
  (bind _rotation_2 (Math|Transform|BreakTransform _returnvalue_2))
  (bind _returnvalue_3 (Math|Vector|GetForwardVector _rotation))
  (bind _returnvalue_4 (Math|Vector|GetForwardVector _rotation_2))
  (bind (_x _y) (Math|Vector|BreakVector _returnvalue_4))
  (bind _returnvalue_5 (* _returnvalue_3 -1e+01))
  (bind (_x_2 _y_2) (Math|Vector|BreakVector _returnvalue_5))
  ;[1 1 1] Camera Movement
  ;;[1 1 1] Move Right
  (:Pressed
    (Variables|Default|SetMoveRight true)
    (Variables|Default|SetActorSelected 0)
    (if (Variables|Default|GetMoveRight)
      (Pawn|Input|AddMovementInput (Math|Vector|GetRightVector (.Rotation (Math|Transform|BreakTransform (Transformation|GetWorldTransform (Variables|Default|Getcameraarm))))) 1.0 false))
    ;;[1 1 1] Move Forward
    (if (Variables|Default|GetForward)
      (Pawn|Input|AddMovementInput (Math|Vector|Normalize (Math|Vector|MakeVector _x _y 0.0)) 1.0 false))
    ;;[1 1 1] Move Back
    (if (Variables|Default|GetBack)
      (Pawn|Input|AddMovementInput (Math|Vector|Normalize (Math|Vector|MakeVector _x_2 _y_2 0.0)) 1.0 false)))
  (:Released
    (Variables|Default|SetMoveRight false)))

(event Input|KeyboardEvents|W
  (params (Key :type Key%20Structure :default "AnyKey"))
  (bind _cameraarm (Variables|Default|Getcameraarm))
  (bind _cameraarm_2 (Variables|Default|Getcameraarm))
  (bind _returnvalue (Transformation|GetWorldTransform _cameraarm))
  (bind _returnvalue_2 (Transformation|GetWorldTransform _cameraarm_2))
  (bind _rotation (Math|Transform|BreakTransform _returnvalue))
  (bind _rotation_2 (Math|Transform|BreakTransform _returnvalue_2))
  (bind _returnvalue_3 (Math|Vector|GetForwardVector _rotation))
  (bind _returnvalue_4 (Math|Vector|GetForwardVector _rotation_2))
  (bind (_x _y) (Math|Vector|BreakVector _returnvalue_4))
  (bind _returnvalue_5 (* _returnvalue_3 -1e+01))
  (bind (_x_2 _y_2) (Math|Vector|BreakVector _returnvalue_5))
  ;[1 1 1] Camera Movement
  ;;[1 1 1] Move Forward
  (:Pressed
    (Variables|Default|SetForward true)
    (Variables|Default|SetActorSelected 0)
    (if (Variables|Default|GetForward)
      (Pawn|Input|AddMovementInput (Math|Vector|Normalize (Math|Vector|MakeVector _x _y 0.0)) 1.0 false))
    ;;[1 1 1] Move Back
    (if (Variables|Default|GetBack)
      (Pawn|Input|AddMovementInput (Math|Vector|Normalize (Math|Vector|MakeVector _x_2 _y_2 0.0)) 1.0 false)))
  (:Released
    (Variables|Default|SetForward false)))

(event Input|KeyboardEvents|S
  (params (Key :type Key%20Structure :default "AnyKey"))
  (bind _cameraarm (Variables|Default|Getcameraarm))
  (bind _returnvalue (Transformation|GetWorldTransform _cameraarm))
  (bind _rotation (Math|Transform|BreakTransform _returnvalue))
  (bind _returnvalue_2 (Math|Vector|GetForwardVector _rotation))
  (bind _returnvalue_3 (* _returnvalue_2 -1e+01))
  (bind (_x _y) (Math|Vector|BreakVector _returnvalue_3))
  ;[1 1 1] Camera Movement
  ;;[1 1 1] Move Back
  (:Pressed
    (Variables|Default|SetBack true)
    (Variables|Default|SetActorSelected 0)
    (if (Variables|Default|GetBack)
      (Pawn|Input|AddMovementInput (Math|Vector|Normalize (Math|Vector|MakeVector _x _y 0.0)) 1.0 false)))
  (:Released
    (Variables|Default|SetBack false)))

(fn ConstructionScript
  (Variables|Default|SetTargetArmLength (Variables|/Script/Engine.SpringArmComponent|GetTargetArmLength (Variables|Default|Getcameraarm))))